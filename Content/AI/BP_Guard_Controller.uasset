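; Guard AI controller that runs BT_Guard on possession and feeds player perception into the blackboard.
; Sensing an actor tagged Player cancels the forget timer, sets HasLineOfSight and stores the actor as EnemyActor.
; Losing the player records the stimulus location as last known position and starts a LineOfSightTimer delay.
; When that delay expires, it clears both line of sight and enemy, giving guards a grace period before forgetting.
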(event `self.ReceivePossess`
  (params (PossessedPawn :type "Pawn Object Reference"))
  (`self.RunBehaviorTree` "/Game/AI/BT_Guard.BT_Guard"))

(event `self.AIPerception.OnTargetPerceptionUpdated`
  (params (Actor :type "Actor Object Reference") (Stimulus :type "AIStimulus Structure"))
  (bind (_age _expirationage _strength _stimuluslocation _receiverlocation _tag _bsuccessfullysensed) (break `AIStimulus` Stimulus))
  (bind _blackboard (`self.Blackboard`))
  (if (`self.ActorHasTag` Actor "Player")
    (if _bsuccessfullysensed
      (`KismetSystemLibrary.K2_ClearAndInvalidateTimerHandle` (`self.EnemyTimer`))
      (`BlackboardComponent.SetValueAsBool` _blackboard (`self.HasLineOfSight`) true)
      (`BlackboardComponent.SetValueAsObject` _blackboard (`self.EnemyActor`) Actor)
      (else
        (`BlackboardComponent.SetValueAsVector` (`self.Blackboard`) (`self.LastKnownPositionKeyName`) _stimuluslocation)
        (bind _returnvalue (`KismetSystemLibrary.K2_SetTimerDelegate` (delegate `StartEnemyTimer`) (`self.Line Of Sight Timer`)))
        (set `self.EnemyTimer` _returnvalue)))))

(event `StartEnemyTimer`
  (bind _blackboard (`self.Blackboard`))
  (`BlackboardComponent.SetValueAsBool` _blackboard (`self.HasLineOfSight`) false)
  (`BlackboardComponent.SetValueAsObject` _blackboard (`self.EnemyActor`) null))

(fn `UserConstructionScript`)